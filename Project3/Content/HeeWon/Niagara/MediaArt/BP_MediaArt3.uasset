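; BP_MediaArt3 is a media art actor whose Niagara effect plays once when an overlap occurs during the game's State3.
; The effect is deactivated on BeginPlay.
; On overlap, it casts the game state to GSC and, if State3 is set, activates the Niagara system, waits briefly, then destroys itself.
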(event `self.ReceiveBeginPlay`
  (`ActorComponent.SetActive` (`self.Niagara`) false false))

(event `/Game/HeeWon/BP/BPI_Interaction.Overlap`
  (bind _asgsc (cast `/Game/HeeWon/BP/GSC` (`GameplayStatics.GetGameState`)))
  (if (`/Game/HeeWon/BP/GSC.state3?` _asgsc)
    (`ActorComponent.SetActive` (`self.Niagara`) true false)
    (`KismetSystemLibrary.Delay` 3.0)
    (`self.K2_DestroyActor`)))

(fn `UserConstructionScript`)