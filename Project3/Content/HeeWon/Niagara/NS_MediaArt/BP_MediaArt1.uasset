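; BP_MediaArt1 is a media art actor that reveals a Niagara effect once the game state reaches its second state.
; The effect starts hidden on BeginPlay, and Tick polls the State2 flag on the GSC game state.
; When the flag is set, a DoOnce shows the effect and plays a timeline that drives the Niagara "Drag" float parameter.
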(event `self.ReceiveBeginPlay`
  (`SceneComponent.SetVisibility` (`self.Niagara`) false false))

(event `self.ReceiveTick`
  (params (DeltaSeconds :type "Float (single-precision)"))
  (bind _asgsc (cast `/Game/HeeWon/BP/GSC` (`GameplayStatics.GetGameState`)))
  (if (`/Game/HeeWon/BP/GSC.state2?` _asgsc)
    (`/Engine/EditorBlueprintResources/StandardMacros.DoOnce` false
      (:`Completed`
        (`SceneComponent.SetVisibility` (`self.Niagara`) true false)
        (bind (_direction _drag) (`Timeline|Drag`)
          (:`Update`
            (`NiagaraComponent.SetVariableFloat` (`self.Niagara`) "Drag" _drag)))))))

(fn `UserConstructionScript`)