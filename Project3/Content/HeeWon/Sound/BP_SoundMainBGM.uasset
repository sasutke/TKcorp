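; BP_SoundMainBGM is an actor that sequences the main background music by spawning and stopping audio components.
; BeginPlay plays two tracks in turn on timed delays.
; A BP_FirstPersonCharacter overlap swaps the second track for a third after a short delay, then destroys the Box trigger.
; Tick polls the GSC game state and, once State5 is true, makes a one-time delayed switch from the third track to a final one.
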(event `self.ReceiveBeginPlay`
  (`KismetSystemLibrary.Delay` 7.0)
  (bind _returnvalue (`AddComponent|NODE_AddAudioComponent-6`))
  (`KismetSystemLibrary.Delay` 27.0)
  (`AudioComponent.Stop` _returnvalue)
  (`KismetSystemLibrary.Delay` 7.0)
  (bind _returnvalue_2 (`AddComponent|NODE_AddAudioComponent-4`)))

(event `self.ReceiveActorBeginOverlap`
  (params (OtherActor :type "Actor Object Reference"))
  (cast `/Game/FirstPerson/Blueprints/BP_FirstPersonCharacter` OtherActor)
  (`KismetSystemLibrary.Delay` 2.0)
  (`AudioComponent.Stop` (stale `self.ReceiveBeginPlay` _returnvalue_2))
  (bind _returnvalue (`AddComponent|NODE_AddAudioComponent-3`))
  (`ActorComponent.K2_DestroyComponent` (`self.Box`)))

(event `self.ReceiveTick`
  (params (DeltaSeconds :type "Float (single-precision)"))
  (bind _asgsc (cast `/Game/HeeWon/BP/GSC` (`GameplayStatics.GetGameState`)))
  (if (`/Game/HeeWon/BP/GSC.state5?` _asgsc)
    (`/Engine/EditorBlueprintResources/StandardMacros.DoOnce` false
      (:`Completed`
        (`KismetSystemLibrary.Delay` 1.0)
        (`AudioComponent.Stop` (stale `self.ReceiveActorBeginOverlap` _returnvalue))
        (`AddComponent|NODE_AddAudioComponent-8`)))))

(fn `UserConstructionScript`)