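; Blood-flow decal actor that animates blood when its Overlap event fires during the game state's third phase (GSC State3).
; BeginPlay creates one dynamic M_Blood material shared by two decals.
; A timeline drives that material's BloodFlow parameter, and a DoOnce removes the Box component on its first update.
; An unconnected timeline graph for moving and rotating a plane, then destroying the actor, never runs.
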(event `self.ReceiveBeginPlay`
  ; 다이나믹 머트리얼
  (bind _returnvalue (`KismetMaterialLibrary.CreateDynamicMaterialInstance` "/Game/HeeWon/MasterMaterial/M_Blood.M_Blood"))
  (bind _output_get (set `self.dynamicMaterial` _returnvalue))
  (`DecalComponent.SetDecalMaterial` (`self.Decal`) _output_get)
  (`DecalComponent.SetDecalMaterial` (`self.Decal1`) _output_get))

(event `/Game/HeeWon/BP/BPI_Interaction.Overlap`
  (`|ExecutionSequence`
    (:`then_0`
      ; 3페 피흐르기
      (bind _asgsc (cast `/Game/HeeWon/BP/GSC` (`GameplayStatics.GetGameState`)))
      (if (`/Game/HeeWon/BP/GSC.state3?` _asgsc)
        (bind (_direction _bloodflow) (`Timeline|Timeline`)
          (:`Update`
            (`MaterialInstanceDynamic.SetScalarParameterValue` (`self.dynamicMaterial`) "BloodFlow" _bloodflow)
            (`/Engine/EditorBlueprintResources/StandardMacros.DoOnce` false
              (:`Completed`
                (`ActorComponent.K2_DestroyComponent` (`self.Box`))))))))))

(fn `UserConstructionScript`)