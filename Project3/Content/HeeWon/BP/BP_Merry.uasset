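; BP_Merry is an interactable painting that shows dialogue and advances story state.
; Tick turns its prompt widget's yaw toward the camera and, once GSC.State3 is set, swaps the plane to MI_Merry and changes the dialogue to mention the girl inside.
; Fkey toggles a WBP_Talk widget and sets State4 if State3 is active.
; EndOverlap removes all widgets and resets the talk flags.
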(event `self.ReceiveBeginPlay`)

(event `self.ReceiveTick`
  (params (DeltaSeconds :type "Float (single-precision)"))
  (`|ExecutionSequence`
    (:`then_0`
      ; 위젯이 항상 나를 쳐다보게
      (`SceneComponent.K2_SetWorldRotation` (`self.Widget`) (`KismetMathLibrary.MakeRotator` 0.0 0.0 (+ (.yaw (`KismetMathLibrary.FindLookAtRotation` (`PlayerCameraManager.GetCameraLocation` (`GameplayStatics.GetPlayerCameraManager` 0)) (`self.K2_GetActorLocation`))) 180.0)) false false))
    (:`then_1`
      (bind _asgsc (cast `/Game/HeeWon/BP/GSC` (`GameplayStatics.GetGameState`)))
      (if (`/Game/HeeWon/BP/GSC.state3?` _asgsc)
        (`/Engine/EditorBlueprintResources/StandardMacros.DoOnce` false
          (:`Completed`
            (set `self.talk` "아까 봤던 소녀가 그림 안에 있다.")
            (`PrimitiveComponent.SetMaterial` (`self.Plane`) 0 "/Game/HeeWon/Drawing/MI_Merry.MI_Merry")))))))

(event `/Game/HeeWon/BP/BPI_Interaction.Fkey`
  (`|ExecutionSequence`
    (:`then_0`
      ; UI인터렉션0번
      (if (`self.ExistWBPTalk`)
        (`Widget.RemoveFromParent` (stale _returnvalue))
        (set `self.ExistWBPTalk` false)
        (else
          (bind _returnvalue (`|CreateWidget` "/Game/HeeWon/Widget/WBP_Talk.WBP_Talk_C" null (`self.name`) (`self.talk`) (`self.Texture_0`)))
          (`UserWidget.AddToViewport` _returnvalue 0)
          (set `self.ExistWBPTalk` true))))
    (:`then_1`
      (bind _asgsc (cast `/Game/HeeWon/BP/GSC` (`GameplayStatics.GetGameState`)))
      (if (`/Game/HeeWon/BP/GSC.state3?` _asgsc)
        (set `/Game/HeeWon/BP/GSC.state4?` true _asgsc)))))

(event `/Game/HeeWon/BP/BPI_Interaction.EndOverlap`
  (`WidgetLayoutLibrary.RemoveAllWidgets`)
  ; 엔드오버랩되면 UI꺼지게
  (set `self.ExistWBPTalk` false)
  (set `self.ExistWBPTalk1` false))

(fn `UserConstructionScript`)