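; BP_Picturename_Long is a picture label Blueprint that displays a name, picture text and year, apparently as a long-title variant with a second picture text field.
; On BeginPlay it copies four variables into the Name, Picture, Year and Picture1 text components.
; The construction script is empty, so this Blueprint only applies those values once play begins.
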(event `self.ReceiveBeginPlay`
  (`TextRenderComponent.K2_SetText` (`self.Name`) (`self.name_var`))
  (`TextRenderComponent.K2_SetText` (`self.Picture`) (`self.Picture_var`))
  (`TextRenderComponent.K2_SetText` (`self.Year`) (`self.Year_var`))
  (`TextRenderComponent.K2_SetText` (`self.Picture1`) (`self.Picture_var_1`)))

(fn `UserConstructionScript`)