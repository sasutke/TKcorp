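; BP_DoorClose is a story trigger that plays a door-closing sound and shows a talk dialogue while the game state's State2 flag is set.
; Overlap disables player movement and, after a short delay, opens WBP_Talk with the actor's name, text and texture.
; Fkey closes the dialogue and restores walking.
; EndOverlap clears all widgets and destroys the actor, with every event gated on the same GSC flag.
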(event `/Game/HeeWon/BP/BPI_Interaction.Overlap`
  (bind _asgsc (cast `/Game/HeeWon/BP/GSC` (`GameplayStatics.GetGameState`)))
  (if (`/Game/HeeWon/BP/GSC.state2?` _asgsc)
    (`GameplayStatics.PlaySoundAtLocation` "/Game/HeeWon/Sound/SC_CloseDoor.SC_CloseDoor" (0.0 0.0 0.0) (struct) 1.0 1.0 0.0 null null null null)
    (`CharacterMovementComponent.SetMovementMode` (`Character.CharacterMovement` (`GameplayStatics.GetPlayerCharacter` 0)) "MOVE_None" 0)
    (`KismetSystemLibrary.Delay` 1.0)
    (bind _returnvalue (`|CreateWidget` "/Game/HeeWon/Widget/WBP_Talk.WBP_Talk_C" null (`self.Name`) (`self.Full Text`) (`self.Texture`)))
    (`UserWidget.AddToViewport` _returnvalue 0)))

(event `/Game/HeeWon/BP/BPI_Interaction.Fkey`
  (bind _asgsc (cast `/Game/HeeWon/BP/GSC` (`GameplayStatics.GetGameState`)))
  (if (`/Game/HeeWon/BP/GSC.state2?` _asgsc)
    (`Widget.RemoveFromParent` (stale `/Game/HeeWon/BP/BPI_Interaction.Overlap` _returnvalue))
    (`CharacterMovementComponent.SetMovementMode` (`Character.CharacterMovement` (`GameplayStatics.GetPlayerCharacter` 0)) "MOVE_Walking" 0)))

(event `/Game/HeeWon/BP/BPI_Interaction.EndOverlap`
  (bind _asgsc (cast `/Game/HeeWon/BP/GSC` (`GameplayStatics.GetGameState`)))
  (if (`/Game/HeeWon/BP/GSC.state2?` _asgsc)
    (`WidgetLayoutLibrary.RemoveAllWidgets`)
    (`self.K2_DestroyActor`)))

(fn `UserConstructionScript`
  (`parent.UserConstructionScript`))