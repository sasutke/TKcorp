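; BP_BasicCollision is a collision actor that reveals a decal on overlap while the GSC game state's State2 flag is set.
; The decal is hidden shortly after BeginPlay, and an overlap makes it visible when the flag is true.
; Ending the overlap under the same flag destroys the Box component, and nothing in the graph hides the decal again.
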(event `self.ReceiveBeginPlay`
  (`KismetSystemLibrary.Delay` 0.2)
  (`SceneComponent.SetVisibility` (`self.Decal`) false false))

(event `/Game/HeeWon/BP/BPI_Interaction.Overlap`
  (bind _asnew_blueprint_1 (cast `/Game/HeeWon/BP/GSC` (`GameplayStatics.GetGameState`)))
  (if (`/Game/HeeWon/BP/GSC.state2` _asnew_blueprint_1)
    (`SceneComponent.SetVisibility` (`self.Decal`) true false)))

(event `/Game/HeeWon/BP/BPI_Interaction.EndOverlap`
  (bind _asnew_blueprint_1 (cast `/Game/HeeWon/BP/GSC` (`GameplayStatics.GetGameState`)))
  (if (`/Game/HeeWon/BP/GSC.state2` _asnew_blueprint_1)
    (`ActorComponent.K2_DestroyComponent` (`self.Box`))))

(fn `UserConstructionScript`)