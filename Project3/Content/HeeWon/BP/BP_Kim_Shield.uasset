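; BP_Kim_Shield is a shield barrier linked to BP_Kim that also offers a talk interaction, both active during game state State3.
; The hidden plane gains visibility and collision when the player enters Box, while a timeline animates its material's Shield parameter.
; Tick disables it once Kim's DestroyedSheild flag is set and yaw-billboards the prompt widget to the camera.
; Overlap events show or hide that prompt, and Fkey toggles a WBP_Talk dialogue.
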(event `self.ReceiveBeginPlay`
  (bind _plane (`self.Plane`))
  (bind _returnvalue (`KismetMaterialLibrary.CreateDynamicMaterialInstance` "/Game/HeeWon/MasterMaterial/M_Kim_Shield.M_Kim_Shield"))
  (`PrimitiveComponent.SetMaterial` _plane 0 _returnvalue)
  (`SceneComponent.SetVisibility` _plane false false)
  (`PrimitiveComponent.SetCollisionEnabled` _plane "NoCollision")
  (bind _returnvalue_2 (`GameplayStatics.GetActorOfClass` "/Game/HeeWon/BP/BP_Kim.BP_Kim_C"))
  (set `self.kim` _returnvalue_2))

(event `self.ReceiveTick`
  (params (DeltaSeconds :type "Float (single-precision)"))
  (bind _plane (`self.Plane`))
  (`|ExecutionSequence`
    (:`then_0`
      (if (`/Game/HeeWon/BP/BP_Kim.destroyedSheild?` (`self.kim`))
        (`/Engine/EditorBlueprintResources/StandardMacros.DoOnce` false
          (:`Completed`
            (`SceneComponent.SetVisibility` _plane false false)
            (`PrimitiveComponent.SetCollisionEnabled` _plane "NoCollision")
            (`ActorComponent.K2_DestroyComponent` (`self.Box1`))))))
    (:`then_1`
      ; 위젯이 항상 나를 쳐다보게
      (`SceneComponent.K2_SetWorldRotation` (`self.Widget`) (`KismetMathLibrary.MakeRotator` 0.0 0.0 (+ (.yaw (`KismetMathLibrary.FindLookAtRotation` (`PlayerCameraManager.GetCameraLocation` (`GameplayStatics.GetPlayerCameraManager` 0)) (`self.K2_GetActorLocation`))) 180.0)) false false))))

(event `self.Box.OnComponentBeginOverlap`
  (params (OverlappedComponent :type "PrimitiveComponent Object Reference") (OtherActor :type "Actor Object Reference") (OtherComp :type "PrimitiveComponent Object Reference") (OtherBodyIndex :type Integer) (bFromSweep :type Boolean) (SweepResult :type "HitResult Structure (by ref)"))
  (bind _plane (`self.Plane`))
  (cast `/Game/FirstPerson/Blueprints/BP_FirstPersonCharacter` OtherActor)
  (bind _asgsc (cast `/Game/HeeWon/BP/GSC` (`GameplayStatics.GetGameState`)))
  (if (`/Game/HeeWon/BP/GSC.state3?` _asgsc)
    (`SceneComponent.SetVisibility` _plane true false)
    (`PrimitiveComponent.SetCollisionEnabled` _plane "QueryAndPhysics")
    (`ActorComponent.K2_DestroyComponent` (`self.Box`))
    (bind (_direction _newtrack_0) (`Timeline|Shield` :!via `PlayFromStart`)
      (:`Update`
        (`MeshComponent.SetScalarParameterValueOnMaterials` (`self.Plane`) "Shield" _newtrack_0)
        (set `self.shieldOn?` true)))))

(event `/Game/HeeWon/BP/BPI_Interaction.Overlap`
  (bind _asgsc (cast `/Game/HeeWon/BP/GSC` (`GameplayStatics.GetGameState`)))
  (if (`/Game/HeeWon/BP/GSC.state3?` _asgsc)
    (`SceneComponent.SetVisibility` (`self.Widget`) true false)))

(event `/Game/HeeWon/BP/BPI_Interaction.EndOverlap`
  (bind _asgsc (cast `/Game/HeeWon/BP/GSC` (`GameplayStatics.GetGameState`)))
  (if (`/Game/HeeWon/BP/GSC.state3?` _asgsc)
    (`WidgetLayoutLibrary.RemoveAllWidgets`)
    (`SceneComponent.SetVisibility` (`self.Widget`) false false)
    ; 엔드오버랩되면 UI꺼지게
    (set `self.ExistWBPTalk` false)
    (set `self.ExistWBPTalk1` false)))

(event `/Game/HeeWon/BP/BPI_Interaction.Fkey`
  (bind _asgsc (cast `/Game/HeeWon/BP/GSC` (`GameplayStatics.GetGameState`)))
  (if (`/Game/HeeWon/BP/GSC.state3?` _asgsc)
    ; UI인터렉션0번
    (if (`self.ExistWBPTalk`)
      (`Widget.RemoveFromParent` (stale _returnvalue))
      (set `self.ExistWBPTalk` false)
      (else
        (bind _returnvalue (`|CreateWidget` "/Game/HeeWon/Widget/WBP_Talk.WBP_Talk_C" null (`self.name`) (`self.talk`) (`self.Texture_0`)))
        (`UserWidget.AddToViewport` _returnvalue 0)
        (set `self.ExistWBPTalk` true)))))

(fn `UserConstructionScript`)