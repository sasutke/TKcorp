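; BP_Eye1 is an eyeball actor that turns to follow the player's camera and is tied to phase 2 of the game.
; Every tick it rotates the Eye component on yaw only, using a look-at rotation from camera to actor with an offset.
; Tick also watches State2 on the GSC game state and shows the eye once through a DoOnce.
; BeginPlay also sets the eye visible, although its comment says it starts hidden.
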(event `self.ReceiveBeginPlay`
  ; 시작하면 안보이게
  (`SceneComponent.SetVisibility` (`self.Eye`) true false))

(event `self.ReceiveTick`
  (params (DeltaSeconds :type "Float (single-precision)"))
  (`|ExecutionSequence`
    (:`then_0`
      ; 틱마다 눈알이 카메라 따라오게
      (`SceneComponent.K2_SetWorldRotation` (`self.Eye`) (`KismetMathLibrary.MakeRotator` 0.0 0.0 (+ (.yaw (`KismetMathLibrary.FindLookAtRotation` (`PlayerCameraManager.GetCameraLocation` (`GameplayStatics.GetPlayerCameraManager` 0)) (`self.K2_GetActorLocation`))) 270.0)) false false))
    (:`then_1`
      ; 페이즈 2가되면 보이게
      (bind _asgsc (cast `/Game/HeeWon/BP/GSC` (`GameplayStatics.GetGameState`)))
      (if (`/Game/HeeWon/BP/GSC.state2?` _asgsc)
        (`/Engine/EditorBlueprintResources/StandardMacros.DoOnce` false
          (:`Completed`
            (`|ExecutionSequence`
              (:`then_0`
                (`SceneComponent.SetVisibility` (`self.Eye`) true false)))))))))

(fn `UserConstructionScript`)