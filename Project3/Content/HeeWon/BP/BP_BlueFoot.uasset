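; BP_BlueFoot is an actor whose drawing plane fades its color saturation in response to game state.
; On BeginPlay it creates a dynamic instance of MI_Drawing17 on the Plane.
; Tick polls the GSC game state, and once State3 is true a DoOnce starts a timeline.
; The timeline drives the BaseColorSaturate material parameter.
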(event `self.ReceiveBeginPlay`
  (`PrimitiveComponent.CreateDynamicMaterialInstance` (`self.Plane`) 0 "/Game/HeeWon/Drawing/MI_Drawing17.MI_Drawing17" "None"))

(event `self.ReceiveTick`
  (params (DeltaSeconds :type "Float (single-precision)"))
  (bind _asgsc (cast `/Game/HeeWon/BP/GSC` (`GameplayStatics.GetGameState`)))
  (if (`/Game/HeeWon/BP/GSC.state3?` _asgsc)
    (`/Engine/EditorBlueprintResources/StandardMacros.DoOnce` false
      (:`Completed`
        (bind (_direction _newtrack_0) (`Timeline|Timeline` :!via `PlayFromStart`)
          (:`Update`
            (`MeshComponent.SetScalarParameterValueOnMaterials` (`self.Plane`) "BaseColorSaturate" _newtrack_0)))))))

(fn `UserConstructionScript`)