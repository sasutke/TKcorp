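; Interactable NPC actor with three skeletal meshes that shows dialogue on its Fkey event and destroys itself once game state GSC reports State2.
; Overlap enables custom depth and feeds a timeline-animated outline material into a post process; leaving disables the highlight and removes all widgets.
; Fkey toggles WBP_Talk according to NPeople, with a two-page variant, and plays an optional animation on one mesh.
; Tick yaws the press-F widget toward the camera.
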(event `self.ReceiveBeginPlay`
  (`|ExecutionSequence`
    (:`then_0`
      ; 시작하자마자 다이나믹 머트리얼 인스턴스 생성
      (bind _returnvalue (`KismetMaterialLibrary.CreateDynamicMaterialInstance` "/Game/HeeWon/MasterMaterial/MI_EdgeOutline_Test.MI_EdgeOutline_Test"))
      (set `self.Outliner` _returnvalue))))

(event `self.ReceiveTick`
  (params (DeltaSeconds :type "Float (single-precision)"))
  (`|ExecutionSequence`
    (:`then_0`
      ; 위젯이 항상 나를 쳐다보게
      (`SceneComponent.K2_SetWorldRotation` (`self.WBP_PressF`) (`KismetMathLibrary.MakeRotator` 0.0 0.0 (+ (.yaw (`KismetMathLibrary.FindLookAtRotation` (`PlayerCameraManager.GetCameraLocation` (`GameplayStatics.GetPlayerCameraManager` 0)) (`self.K2_GetActorLocation`))) 180.0)) false false))
    (:`then_1`
      ; 2페이즈 되면 파괴
      (bind _asgsc (cast `/Game/HeeWon/BP/GSC` (`GameplayStatics.GetGameState`)))
      (if (`/Game/HeeWon/BP/GSC.state2?` _asgsc)
        (`self.K2_DestroyActor`)))))

(event `self.Overlap`
  (bind _outliner (`self.Outliner`))
  (bind _weightedblendables_array (break `WeightedBlendables` (break `PostProcessSettings` (`PostProcessVolume.Settings` (`self.postprocess`)))))
  ; 트리거박스에 들어갔을때 위젯, 아웃라이너가 보이게
  (`|ExecutionSequence`
    (:`then_0`
      (`PrimitiveComponent.SetRenderCustomDepth` (`self.SKM_Quinn_Simple`) true)
      (`PrimitiveComponent.SetRenderCustomDepth` (`self.SKM_Quinn_Simple1`) true)
      (`PrimitiveComponent.SetRenderCustomDepth` (`self.SKM_Quinn_Simple2`) true))
    (:`then_1`
      (bind (_direction _intensity) (`Timeline|Outline Intensity` :!label _label)
        (:`Update`
          (`MaterialInstanceDynamic.SetScalarParameterValue` _outliner "LineWidth" _intensity))))
    (:`then_2`
      (`KismetArrayLibrary.Array_Set` _weightedblendables_array 0 (make `WeightedBlendable` 1.0 _outliner)))))

(event `self.EndOverlap`
  ; 트리거박스에 들어갔을때 위젯, 아웃라이너가 보이게
  (`WidgetLayoutLibrary.RemoveAllWidgets`)
  (`|ExecutionSequence`
    (:`then_0`
      (goto _label :!via `Stop`))
    (:`then_1`
      (`PrimitiveComponent.SetRenderCustomDepth` (`self.SKM_Quinn_Simple`) false)
      (`PrimitiveComponent.SetRenderCustomDepth` (`self.SKM_Quinn_Simple1`) false)
      (`PrimitiveComponent.SetRenderCustomDepth` (`self.SKM_Quinn_Simple2`) false)
      ;; 엔드오버랩되면 UI꺼지게
      (set `self.ExistWBPTalk` false)
      (set `self.ExistWBPTalk1` false))))

(event `self.Fkey`
  (switch `int` (`self.NPeople`)
    (:`0`
      ; UI인터렉션0번
      (if (`self.ExistWBPTalk`)
        (`Widget.RemoveFromParent` (stale _returnvalue))
        (set `self.ExistWBPTalk` false)
        (else
          (bind _returnvalue (`|CreateWidget` "/Game/HeeWon/Widget/WBP_Talk.WBP_Talk_C" null (`self.name`) (`self.talk`) (`self.Texture_0`)))
          (`UserWidget.AddToViewport` _returnvalue 0)
          (set `self.ExistWBPTalk` true)
          (`/Engine/EditorBlueprintResources/StandardMacros.IsValid` (`self.New Anim to Play`)
            (:`Is Valid`
              (`SkeletalMeshComponent.PlayAnimation` (`self.SKM_Quinn_Simple`) (`self.New Anim to Play`) false))))))
    (:`1`
      ; UI인터렉션1번
      (if (`self.ExistWBPTalk`)
        (if (`self.ExistWBPTalk1`)
          (`Widget.RemoveFromParent` (stale _returnvalue_2))
          (set `self.ExistWBPTalk` false)
          (set `self.ExistWBPTalk1` false)
          (else
            (`Widget.RemoveFromParent` (stale _returnvalue_3))
            (bind _returnvalue_2 (`|CreateWidget` "/Game/HeeWon/Widget/WBP_Talk.WBP_Talk_C" null (`self.name`) (`self.Talk2`) (`self.Texture`)))
            (`UserWidget.AddToViewport` _returnvalue_2 0)
            (set `self.ExistWBPTalk1` true)))
        (else
          (bind _returnvalue_3 (`|CreateWidget` "/Game/HeeWon/Widget/WBP_Talk.WBP_Talk_C" null (`self.name`) (`self.talk`) (`self.Texture_0`)))
          (`UserWidget.AddToViewport` _returnvalue_3 0)
          (set `self.ExistWBPTalk` true)
          (`/Engine/EditorBlueprintResources/StandardMacros.IsValid` (`self.New Anim to Play`)
            (:`Is Valid`
              (`SkeletalMeshComponent.PlayAnimation` (`self.SKM_Quinn_Simple`) (`self.New Anim to Play`) false))))))
    (:`2`
      ; UI인터렉션 2번
      (if (`self.ExistWBPTalk`)
        (`Widget.RemoveFromParent` (stale _returnvalue_4))
        (set `self.ExistWBPTalk` false)
        (else
          (bind _returnvalue_4 (`|CreateWidget` "/Game/HeeWon/Widget/WBP_Talk.WBP_Talk_C" null (`self.name`) (`self.talk`) (`self.Texture_0`)))
          (`UserWidget.AddToViewport` _returnvalue_4 0)
          (set `self.ExistWBPTalk` true)
          (`/Engine/EditorBlueprintResources/StandardMacros.IsValid` (`self.New Anim to Play`)
            (:`Is Valid`
              (`SkeletalMeshComponent.PlayAnimation` (`self.SKM_Quinn_Simple`) (`self.New Anim to Play`) false))))))))

(fn `UserConstructionScript`)