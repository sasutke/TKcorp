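; BP_SecondFloorCollision is a trigger that starts the second-floor phase of the game when its box is overlapped.
; On overlap it sets State2 on the GSC game state and plays a timeline that adjusts directional light intensity.
; After a three-minute delay, a second timeline drives post-process film grain intensity.
; The box collision is destroyed right after triggering, so it fires once.
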(event `/Game/HeeWon/BP/BPI_Interaction.Overlap`
  (`|ExecutionSequence`
    (:`then_0`
      ; 오버랩 되면 게임모드 2
      (bind _asgsc (cast `/Game/HeeWon/BP/GSC` (`GameplayStatics.GetGameState`)))
      (set `/Game/HeeWon/BP/GSC.state2` true _asgsc))
    (:`then_1`
      ; 오버랩 되면조명 조절
      (bind (_direction _lightintensity) (`Timeline|Timeline`)
        (:`Update`
          (`LightComponent.SetIntensity` (`Light.LightComponent` (`self.Direction`)) _lightintensity))))
    (:`then_2`
      ; 3분후 필름그레인
      (`KismetSystemLibrary.Delay` 180.0)
      (bind (_direction_2 _filmgrain) (`Timeline|Timeline_0`)
        (:`Update`
          (setmembers `PostProcessSettings` :`StructRef` (`PostProcessVolume.Settings` (`self.PPV`)) :`FilmGrainIntensity` _filmgrain))))
    (:`then_3`
      ; 박스 컬리전 부수기
      (`ActorComponent.K2_DestroyComponent` (`self.Box`)))))

(fn `UserConstructionScript`)