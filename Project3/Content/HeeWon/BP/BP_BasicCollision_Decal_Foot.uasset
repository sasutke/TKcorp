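; Collision trigger actor that makes a trail of footprint decals appear one after another with sound.
; All thirteen decals are hidden on BeginPlay, and the Overlap event calls ShowFoot, which proceeds only if State5 is set on the GSC game state.
; It then destroys the Box component and reveals the decals through a hardcoded chain of short Delays, adding an audio component at each step.
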(event `self.ReceiveBeginPlay`
  (`SceneComponent.SetVisibility` (`self.Decal6`) false false)
  (`SceneComponent.SetVisibility` (`self.Decal11`) false false)
  (`SceneComponent.SetVisibility` (`self.Decal10`) false false)
  (`SceneComponent.SetVisibility` (`self.Decal9`) false false)
  (`SceneComponent.SetVisibility` (`self.Decal8`) false false)
  (`SceneComponent.SetVisibility` (`self.Decal7`) false false)
  (`SceneComponent.SetVisibility` (`self.Decal12`) false false)
  (`SceneComponent.SetVisibility` (`self.Decal5`) false false)
  (`SceneComponent.SetVisibility` (`self.Decal4`) false false)
  (`SceneComponent.SetVisibility` (`self.Decal3`) false false)
  (`SceneComponent.SetVisibility` (`self.Decal2`) false false)
  (`SceneComponent.SetVisibility` (`self.Decal`) false false)
  (`SceneComponent.SetVisibility` (`self.Decal1`) false false))

(event `ShowFoot`
  ; 오버랩되면 발나오기
  (bind _asgsc (cast `/Game/HeeWon/BP/GSC` (`GameplayStatics.GetGameState`)))
  (if (`/Game/HeeWon/BP/GSC.state5?` _asgsc)
    (`ActorComponent.K2_DestroyComponent` (`self.Box`))
    (`SceneComponent.SetVisibility` (`self.Decal`) true false)
    (`AddComponent|NODE_AddAudioComponent-0`)
    (`KismetSystemLibrary.Delay` 0.3)
    (`SceneComponent.SetVisibility` (`self.Decal1`) true false)
    (`AddComponent|NODE_AddAudioComponent-1`)
    (`KismetSystemLibrary.Delay` 0.3)
    (`SceneComponent.SetVisibility` (`self.Decal2`) true false)
    (`AddComponent|NODE_AddAudioComponent-2`)
    (`KismetSystemLibrary.Delay` 0.3)
    (`SceneComponent.SetVisibility` (`self.Decal3`) true false)
    (`AddComponent|NODE_AddAudioComponent-3`)
    (`KismetSystemLibrary.Delay` 0.3)
    (`SceneComponent.SetVisibility` (`self.Decal4`) true false)
    (`AddComponent|NODE_AddAudioComponent-4`)
    (`KismetSystemLibrary.Delay` 0.3)
    (`SceneComponent.SetVisibility` (`self.Decal5`) true false)
    (`AddComponent|NODE_AddAudioComponent-5`)
    (`KismetSystemLibrary.Delay` 0.3)
    (`SceneComponent.SetVisibility` (`self.Decal6`) true false)
    (`AddComponent|NODE_AddAudioComponent-8`)
    (`KismetSystemLibrary.Delay` 0.3)
    (`SceneComponent.SetVisibility` (`self.Decal7`) true false)
    (`AddComponent|NODE_AddAudioComponent-6`)
    (`KismetSystemLibrary.Delay` 0.3)
    (`SceneComponent.SetVisibility` (`self.Decal8`) true false)
    (`AddComponent|NODE_AddAudioComponent-7`)
    (`KismetSystemLibrary.Delay` 0.3)
    (`SceneComponent.SetVisibility` (`self.Decal9`) true false)
    (`AddComponent|NODE_AddAudioComponent-9`)
    (`KismetSystemLibrary.Delay` 0.3)
    (`SceneComponent.SetVisibility` (`self.Decal10`) true false)
    (`AddComponent|NODE_AddAudioComponent-11`)
    (`KismetSystemLibrary.Delay` 0.3)
    (`SceneComponent.SetVisibility` (`self.Decal11`) true false)
    (`AddComponent|NODE_AddAudioComponent-12`)
    (`KismetSystemLibrary.Delay` 0.3)
    (`SceneComponent.SetVisibility` (`self.Decal12`) true false)
    (`AddComponent|NODE_AddAudioComponent-13`)))

(event `/Game/HeeWon/BP/BPI_Interaction.Overlap`
  (`self.ShowFoot`))

(fn `UserConstructionScript`
  (`parent.UserConstructionScript`))