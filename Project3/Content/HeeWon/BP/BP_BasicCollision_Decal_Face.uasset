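; Collision trigger actor that reveals a decal with audio, by its name a face, when the game state allows it.
; The decal is hidden shortly after BeginPlay.
; Its Overlap event checks State3 on the GSC game state, then shows the decal, adds an audio component and destroys the Box so the reveal happens once.
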(event `self.ReceiveBeginPlay`
  (`KismetSystemLibrary.Delay` 0.2)
  (`SceneComponent.SetVisibility` (`self.Decal`) false false))

(event `/Game/HeeWon/BP/BPI_Interaction.Overlap`
  (bind _asgsc (cast `/Game/HeeWon/BP/GSC` (`GameplayStatics.GetGameState`)))
  (if (`/Game/HeeWon/BP/GSC.state3?` _asgsc)
    (`SceneComponent.SetVisibility` (`self.Decal`) true false)
    (`AddComponent|NODE_AddAudioComponent-0`)
    (`ActorComponent.K2_DestroyComponent` (`self.Box`))))

(fn `UserConstructionScript`)