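; Collision trigger that makes hand decals appear one after another when overlapped, as a staged scare or visual effect.
; Eight decals are hidden shortly after BeginPlay, then revealed in a fixed order with irregular short delays on Overlap.
; Both overlap handlers act only while the GSC game state's State3 is true; EndOverlap then destroys the Box component so the trigger is spent.
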(event `self.ReceiveBeginPlay`
  ; 데칼 안보이게하기
  (`KismetSystemLibrary.Delay` 0.01)
  (`SceneComponent.SetVisibility` (`self.Decal`) false false)
  (`SceneComponent.SetVisibility` (`self.Decal2`) false false)
  (`SceneComponent.SetVisibility` (`self.Decal3`) false false)
  (`SceneComponent.SetVisibility` (`self.Decal4`) false false)
  (`SceneComponent.SetVisibility` (`self.Decal5`) false false)
  (`SceneComponent.SetVisibility` (`self.Decal1`) false false)
  (`SceneComponent.SetVisibility` (`self.Decal6`) false false)
  (`SceneComponent.SetVisibility` (`self.Decal7`) false false))

(event `self.Overlap`
  ; 오버랩되면 손나오기
  (bind _asgsc (cast `/Game/HeeWon/BP/GSC` (`GameplayStatics.GetGameState`)))
  (if (`/Game/HeeWon/BP/GSC.state3?` _asgsc)
    (`SceneComponent.SetVisibility` (`self.Decal`) true false)
    (`KismetSystemLibrary.Delay` 0.2)
    (`SceneComponent.SetVisibility` (`self.Decal1`) true false)
    (`KismetSystemLibrary.Delay` 0.1)
    (`SceneComponent.SetVisibility` (`self.Decal2`) true false)
    (`KismetSystemLibrary.Delay` 0.3)
    (`SceneComponent.SetVisibility` (`self.Decal3`) true false)
    (`KismetSystemLibrary.Delay` 0.05)
    (`SceneComponent.SetVisibility` (`self.Decal6`) true false)
    (`KismetSystemLibrary.Delay` 0.3)
    (`SceneComponent.SetVisibility` (`self.Decal4`) true false)
    (`KismetSystemLibrary.Delay` 0.1)
    (`SceneComponent.SetVisibility` (`self.Decal7`) true false)
    (`KismetSystemLibrary.Delay` 0.5)
    (`SceneComponent.SetVisibility` (`self.Decal5`) true false)))

(event `self.EndOverlap`
  (bind _asgsc (cast `/Game/HeeWon/BP/GSC` (`GameplayStatics.GetGameState`)))
  (if (`/Game/HeeWon/BP/GSC.state3?` _asgsc)
    (`ActorComponent.K2_DestroyComponent` (`self.Box`))))

(fn `UserConstructionScript`)