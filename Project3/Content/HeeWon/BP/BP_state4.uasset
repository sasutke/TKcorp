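; BP_state4 is an overlap-driven actor that advances a state flag on the GSC game state.
; On overlap, it sets State4 to true if State3 is already set.
; When the overlap ends with State3 set, it destroys itself, so it acts as a one-shot step in a flag sequence.
; The overlap events do not check which actor triggered them.
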(event `/Game/HeeWon/BP/BPI_Interaction.Overlap`
  (bind _asgsc (cast `/Game/HeeWon/BP/GSC` (`GameplayStatics.GetGameState`)))
  (if (`/Game/HeeWon/BP/GSC.state3?` _asgsc)
    (set `/Game/HeeWon/BP/GSC.state4?` true _asgsc)))

(event `/Game/HeeWon/BP/BPI_Interaction.EndOverlap`
  (bind _asgsc (cast `/Game/HeeWon/BP/GSC` (`GameplayStatics.GetGameState`)))
  (if (`/Game/HeeWon/BP/GSC.state3?` _asgsc)
    (`self.K2_DestroyActor`)))

(fn `UserConstructionScript`
  (`parent.UserConstructionScript`))