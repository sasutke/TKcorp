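; BP_PlayWithMeIB is a scripted scare trigger that makes hand decals appear in sequence on overlap while the GSC game state's State4 flag is set.
; Six decals are revealed one by one with short, uneven delays, each accompanied by a newly added audio component.
; Ending the overlap during State4 destroys the Box component, apparently the trigger volume, so the sequence does not replay.
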(event `/Game/HeeWon/BP/BPI_Interaction.Overlap`
  ; 오버랩되면 손나오기
  (bind _asgsc (cast `/Game/HeeWon/BP/GSC` (`GameplayStatics.GetGameState`)))
  (if (`/Game/HeeWon/BP/GSC.state4?` _asgsc)
    (`SceneComponent.SetVisibility` (`self.Decal`) true false)
    (`AddComponent|NODE_AddAudioComponent-0`)
    (`KismetSystemLibrary.Delay` 0.4)
    (`SceneComponent.SetVisibility` (`self.Decal1`) true false)
    (`AddComponent|NODE_AddAudioComponent-1`)
    (`KismetSystemLibrary.Delay` 0.3)
    (`SceneComponent.SetVisibility` (`self.Decal2`) true false)
    (`AddComponent|NODE_AddAudioComponent-2`)
    (`KismetSystemLibrary.Delay` 0.4)
    (`SceneComponent.SetVisibility` (`self.Decal3`) true false)
    (`AddComponent|NODE_AddAudioComponent-3`)
    (`KismetSystemLibrary.Delay` 0.8)
    (`SceneComponent.SetVisibility` (`self.Decal4`) true false)
    (`AddComponent|NODE_AddAudioComponent-4`)
    (`KismetSystemLibrary.Delay` 0.8)
    (`SceneComponent.SetVisibility` (`self.Decal5`) true false)
    (`AddComponent|NODE_AddAudioComponent-6`)))

(event `/Game/HeeWon/BP/BPI_Interaction.EndOverlap`
  ; 오버랩되면 파괴
  (bind _asgsc (cast `/Game/HeeWon/BP/GSC` (`GameplayStatics.GetGameState`)))
  (if (`/Game/HeeWon/BP/GSC.state4?` _asgsc)
    (`ActorComponent.K2_DestroyComponent` (`self.Box`))))

(fn `UserConstructionScript`)