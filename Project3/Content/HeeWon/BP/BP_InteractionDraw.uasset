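; BP_InteractionDraw is an interactable drawing that shows dialogue on the F key and dissolves as the conversation advances.
; Successive presses show the first WBP_Talk line, lock player input while a timeline drives the dissolve material, show the second line, then close it.
; Tick yaws the PressF prompt toward the camera and destroys the actor when GSC reaches State2.
; Leaving overlap clears widgets and dialogue flags; outline highlight logic is disconnected.
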(event `self.ReceiveBeginPlay`
  ; 시작하자마자 다이나믹 머트리얼 인스턴스 생성
  (bind _returnvalue (`KismetMaterialLibrary.CreateDynamicMaterialInstance` "/Game/HeeWon/Drawing/MI_DissolveDrawing.MI_DissolveDrawing"))
  (set `self.Material` _returnvalue)
  (`PrimitiveComponent.SetMaterial` (`self.Plane`) 0 (`self.Material`))
  (bind _returnvalue_2 (`KismetMaterialLibrary.CreateDynamicMaterialInstance` "/Game/HeeWon/MasterMaterial/MI_EdgeOutline_Test.MI_EdgeOutline_Test"))
  (set `self.Outliner` _returnvalue_2))

(event `self.ReceiveTick`
  (params (DeltaSeconds :type "Float (single-precision)"))
  (`|ExecutionSequence`
    (:`then_0`
      ; 위젯이 항상 나를 쳐다보게
      (`SceneComponent.K2_SetWorldRotation` (`self.Press F`) (`KismetMathLibrary.MakeRotator` 0.0 0.0 (+ (.yaw (`KismetMathLibrary.FindLookAtRotation` (`PlayerCameraManager.GetCameraLocation` (`GameplayStatics.GetPlayerCameraManager` 0)) (`self.K2_GetActorLocation`))) 180.0)) false false))
    (:`then_1`
      ; 2페이즈되면 콜리전 부시기
      (bind _asgsc (cast `/Game/HeeWon/BP/GSC` (`GameplayStatics.GetGameState`)))
      (if (`/Game/HeeWon/BP/GSC.state2?` _asgsc)
        (`/Engine/EditorBlueprintResources/StandardMacros.DoOnce` false
          (:`Completed`
            (`self.K2_DestroyActor`)))))))

(event `/Game/HeeWon/BP/BPI_Interaction.Overlap`)

(event `/Game/HeeWon/BP/BPI_Interaction.EndOverlap`
  ; UI대화
  (`WidgetLayoutLibrary.RemoveAllWidgets`)
  (`|ExecutionSequence`
    (:`then_0`
      ;; 엔드오버랩되면 UI꺼지게
      (set `self.ExistWBPTalk` false)
      (set `self.ExistWBPTalk1` false)
      (set `self.doDrawMove?` false))))

(event `/Game/HeeWon/BP/BPI_Interaction.Fkey`
  (`|ExecutionSequence`
    (:`then_0`
      ; UI인터렉션0번
      (if (`self.ExistWBPTalk`)
        (if (`self.ExistWBPTalk1`)
          (`Widget.RemoveFromParent` (stale _returnvalue))
          (set `self.ExistWBPTalk` false)
          (set `self.ExistWBPTalk1` false)
          (else
            (set `self.doDrawMove?` true)
            (`Widget.RemoveFromParent` (stale _returnvalue_2))
            (`self.DisableInput` (`GameplayStatics.GetPlayerCharacter` 0) (`GameplayStatics.GetPlayerController` 0))
            (`KismetSystemLibrary.Delay` 4.0)
            (`self.EnableInput` (`GameplayStatics.GetPlayerCharacter` 0) (`GameplayStatics.GetPlayerController` 0))
            (bind _returnvalue (`|CreateWidget` "/Game/HeeWon/Widget/WBP_Talk.WBP_Talk_C" null (`self.name`) (`self.Talk2`) null))
            (`UserWidget.AddToViewport` _returnvalue 0)
            (set `self.ExistWBPTalk1` true)
            (set `self.doDrawMove?` false)))
        (else
          (bind _returnvalue_2 (`|CreateWidget` "/Game/HeeWon/Widget/WBP_Talk.WBP_Talk_C" null (`self.name`) (`self.Talk`) null))
          (`UserWidget.AddToViewport` _returnvalue_2 0)
          (set `self.ExistWBPTalk` true))))
    (:`then_1`
      ; 디졸브
      (if (`self.doDrawMove?`)
        (bind (_direction _dissolve) (`Timeline|Timeline_1` :!via `PlayFromStart` :!label _label)
          (:`Update`
            (`MaterialInstanceDynamic.SetScalarParameterValue` (`self.Material`) "Dissolve" _dissolve)))
        (else
          (goto _label :!via `Stop`))))))

(fn `UserConstructionScript`)