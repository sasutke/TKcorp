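; BP_state5 is a one-shot overlap actor that advances the game's progression from State4 to State5.
; On overlap it casts the game state to GSC and sets State5 only if State4 is already true.
; When the overlap ends it destroys itself if State5 is set, so it stays in place until that flag is true.
; Neither event checks which actor overlaps.
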(event `/Game/HeeWon/BP/BPI_Interaction.Overlap`
  (bind _asgsc (cast `/Game/HeeWon/BP/GSC` (`GameplayStatics.GetGameState`)))
  (if (`/Game/HeeWon/BP/GSC.state4?` _asgsc)
    (set `/Game/HeeWon/BP/GSC.state5?` true _asgsc)))

(event `/Game/HeeWon/BP/BPI_Interaction.EndOverlap`
  (bind _asgsc (cast `/Game/HeeWon/BP/GSC` (`GameplayStatics.GetGameState`)))
  (if (`/Game/HeeWon/BP/GSC.state5?` _asgsc)
    (`self.K2_DestroyActor`)))

(fn `UserConstructionScript`
  (`parent.UserConstructionScript`))