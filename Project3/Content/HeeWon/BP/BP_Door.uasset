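; BP_Door is an interactable door that teleports the player to a linked Location actor on F key.
; Interaction stops footsteps, plays a sound, then fades out, teleports with matching rotation and fades in while input is disabled.
; When the GSC game state's State3 is set, the door instead toggles a WBP_Talk message.
; Tick yaws two widgets toward the camera, and ending overlap removes all widgets.
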(event `/Game/HeeWon/BP/BPI_Interaction.Fkey`
  (bind _location (`self.Location`))
  (bind _returnvalue (`self.K2_GetActorRotation` _location))
  (bind _asbp_first_person_character (cast `/Game/FirstPerson/Blueprints/BP_FirstPersonCharacter` (`GameplayStatics.GetPlayerCharacter` 0)))
  (`TimelineComponent.Stop` (`/Game/FirstPerson/Blueprints/BP_FirstPersonCharacter.Footsteps_TL` _asbp_first_person_character))
  (bind _asgsc (cast `/Game/HeeWon/BP/GSC` (`GameplayStatics.GetGameState`)))
  (if (`/Game/HeeWon/BP/GSC.state3?` _asgsc)
    ; 3페이즈 되면 문이 작동 x
    (if (`self.ExistWBPTalk`)
      (`Widget.RemoveFromParent` (stale _returnvalue_2))
      (set `self.ExistWBPTalk` false)
      (else
        (bind _returnvalue_2 (`|CreateWidget` "/Game/HeeWon/Widget/WBP_Talk.WBP_Talk_C" null (`self.name`) (`self.talk`) null))
        (`UserWidget.AddToViewport` _returnvalue_2 0)
        (set `self.ExistWBPTalk` true)))
    (else
      (`GameplayStatics.PlaySound2D` "/Game/HeeWon/Sound/SW_Door.SW_Door" 0.4 1.0 0.0 null null)
      ; F누르면 텔레포트
      (bind _returnvalue_3 (`|CreateWidget` "/Game/HeeWon/Widget/WBP_Fadeout.WBP_Fadeout_C"))
      (bind _output_get (set `self.Fadeout` _returnvalue_3))
      (`UserWidget.AddToViewport` _output_get 0)
      (`self.DisableInput` (`GameplayStatics.GetPlayerCharacter` 0) (`GameplayStatics.GetPlayerController` 0))
      (`KismetSystemLibrary.Delay` 2.0)
      (`Widget.RemoveFromParent` (`self.Fadeout`))
      (`Controller.SetControlRotation` (`GameplayStatics.GetPlayerController` 0) _returnvalue)
      (`self.K2_TeleportTo` (`GameplayStatics.GetPlayerCharacter` 0) (`self.K2_GetActorLocation` _location) _returnvalue)
      (bind _returnvalue_4 (`|CreateWidget` "/Game/HeeWon/Widget/WBP_Fadein.WBP_Fadein_C"))
      (`UserWidget.AddToViewport` _returnvalue_4 0)
      (`KismetSystemLibrary.Delay` 2.0)
      (`Widget.RemoveFromParent` _returnvalue_4)
      (`self.EnableInput` (`GameplayStatics.GetPlayerCharacter` 0) (`GameplayStatics.GetPlayerController` 0)))))

(event `self.ReceiveTick`
  (params (DeltaSeconds :type "Float (single-precision)"))
  (`|ExecutionSequence`
    (:`then_0`
      ; 위젯이 항상 나를 쳐다보게
      (`SceneComponent.K2_SetWorldRotation` (`self.Widget`) (`KismetMathLibrary.MakeRotator` 0.0 0.0 (+ (.yaw (`KismetMathLibrary.FindLookAtRotation` (`PlayerCameraManager.GetCameraLocation` (`GameplayStatics.GetPlayerCameraManager` 0)) (`self.K2_GetActorLocation`))) 180.0)) false false)
      (`SceneComponent.K2_SetWorldRotation` (`self.Widget1`) (`KismetMathLibrary.MakeRotator` 0.0 0.0 (+ (.yaw (`KismetMathLibrary.FindLookAtRotation` (`PlayerCameraManager.GetCameraLocation` (`GameplayStatics.GetPlayerCameraManager` 0)) (`self.K2_GetActorLocation`))) 180.0)) false false))))

(event `/Game/HeeWon/BP/BPI_Interaction.Overlap`)

(event `/Game/HeeWon/BP/BPI_Interaction.EndOverlap`
  ; 오버랩끝났을때 UI
  (`WidgetLayoutLibrary.RemoveAllWidgets`)
  (set `self.ExistWBPTalk` false))

(fn `UserConstructionScript`
  (`parent.UserConstructionScript`))