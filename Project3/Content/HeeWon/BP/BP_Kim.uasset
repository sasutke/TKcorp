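; BP_Kim is an interactable character shown as a material-driven plane that offers dialogue linked to BP_Kim_Shield.
; Tick turns its widget toward the camera, starts material motion on GSC's State2, and fades in emissive and shows the widget when the shield turns on.
; With the shield on, Fkey toggles WBP_Talk; closing the first dialogue sets DestroyedSheild, plays a crash sound, clears the highlight and switches to the second text.
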(event `self.ReceiveBeginPlay`
  (bind _returnvalue (`KismetMaterialLibrary.CreateDynamicMaterialInstance` "/Game/HeeWon/MasterMaterial/M_Kim.M_Kim"))
  (`PrimitiveComponent.SetMaterial` (`self.Plane`) 0 _returnvalue)
  (bind _returnvalue_2 (`GameplayStatics.GetActorOfClass` "/Game/HeeWon/BP/BP_Kim_Shield.BP_Kim_Shield_C"))
  (set `self.kim_shield` _returnvalue_2))

(event `self.ReceiveTick`
  (params (DeltaSeconds :type "Float (single-precision)"))
  (bind _kim_shield (`self.kim_shield`))
  (bind _plane (`self.Plane`))
  (`|ExecutionSequence`
    (:`then_0`
      ; 그림변화
      (bind _asgsc (cast `/Game/HeeWon/BP/GSC` (`GameplayStatics.GetGameState`)))
      (if (`/Game/HeeWon/BP/GSC.state2?` _asgsc)
        (`/Engine/EditorBlueprintResources/StandardMacros.DoOnce` false
          (:`Completed`
            (`MeshComponent.SetScalarParameterValueOnMaterials` _plane "Xspeed" 0.05)
            (`MeshComponent.SetScalarParameterValueOnMaterials` _plane "Yspeed" 0.07)
            (`MeshComponent.SetScalarParameterValueOnMaterials` _plane "Xspeed1" -0.05)))))
    (:`then_1`
      ; 위젯 돌아가게
      (`SceneComponent.K2_SetWorldRotation` (`self.Widget`) (`KismetMathLibrary.MakeRotator` 0.0 0.0 (+ (.yaw (`KismetMathLibrary.FindLookAtRotation` (`PlayerCameraManager.GetCameraLocation` (`GameplayStatics.GetPlayerCameraManager` 0)) (`self.K2_GetActorLocation`))) 180.0)) false false))
    (:`then_2`
      ; 쉴드생성시 이미시브
      (`/Engine/EditorBlueprintResources/StandardMacros.IsValid` _kim_shield
        (:`Is Valid`
          (if (`/Game/HeeWon/BP/BP_Kim_Shield.shieldOn?` _kim_shield)
            (`/Engine/EditorBlueprintResources/StandardMacros.DoOnce` false
              (:`Completed`
                (bind (_direction _newtrack_0) (`Timeline|Emissive` :!via `PlayFromStart`)
                  (:`Update`
                    (`MeshComponent.SetScalarParameterValueOnMaterials` (`self.Plane`) "Emissive" _newtrack_0)
                    (`SceneComponent.SetVisibility` (`self.Widget`) true false)))))))))
    (:`then_3`
      (if (`self.destroyedSheild?`)
        (`/Engine/EditorBlueprintResources/StandardMacros.DoOnce` false
          (:`Completed`
            (`MeshComponent.SetScalarParameterValueOnMaterials` (`self.Plane`) "Emissive" 0.0)
            (`SceneComponent.SetVisibility` (`self.Widget`) false false)))))))

(event `/Game/HeeWon/BP/BPI_Interaction.Overlap`)

(event `/Game/HeeWon/BP/BPI_Interaction.EndOverlap`)

(event `/Game/HeeWon/BP/BPI_Interaction.Fkey`
  (if (`/Game/HeeWon/BP/BP_Kim_Shield.shieldOn?` (`self.kim_shield`))
    (if (`self.destroyedSheild?`)
      ; UI인터렉션0번
      (if (`self.ExistWBPTalk`)
        (`Widget.RemoveFromParent` (stale _returnvalue))
        (set `self.ExistWBPTalk` false)
        (else
          (bind _returnvalue (`|CreateWidget` "/Game/HeeWon/Widget/WBP_Talk.WBP_Talk_C" null (`self.name`) (`self.talk2`) (`self.Texture_0`)))
          (`UserWidget.AddToViewport` _returnvalue 0)
          (set `self.ExistWBPTalk` true)))
      (else
        ; UI인터렉션0번
        (if (`self.ExistWBPTalk`)
          (`Widget.RemoveFromParent` (stale _returnvalue_2))
          (set `self.ExistWBPTalk` false)
          (set `self.destroyedSheild?` true)
          (`GameplayStatics.PlaySoundAtLocation` "/Game/HeeWon/Sound/SC_CrashWindow.SC_CrashWindow" (3753.0 -1478.0 70.0) (struct) 1.0 1.0 0.0 null null null null)
          (else
            (bind _returnvalue_2 (`|CreateWidget` "/Game/HeeWon/Widget/WBP_Talk.WBP_Talk_C" null (`self.name`) (`self.talk`) (`self.Texture_0`)))
            (`UserWidget.AddToViewport` _returnvalue_2 0)
            (set `self.ExistWBPTalk` true)))))))

(fn `UserConstructionScript`)