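; Interactable drawing actor that shows a Press F prompt and outline on overlap, toggles a WBP_Talk dialogue on the F key, and reacts to game phases.
; Overlap enables custom depth and animates an edge-outline post-process material, while Tick turns the prompt toward the camera.
; Tick also polls GSC state: State2 destroys the box and runs a timeline making the dissolve material flow, while State5 activates Niagara effects and a light.
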(event `self.ReceiveBeginPlay`
  ; 시작하자마자 다이나믹 머트리얼 인스턴스 생성
  (bind _returnvalue (`KismetMaterialLibrary.CreateDynamicMaterialInstance` "/Game/HeeWon/MasterMaterial/M_DissolveDrawing.M_DissolveDrawing"))
  (set `self.Material` _returnvalue)
  (`PrimitiveComponent.SetMaterial` (`self.Plane`) 0 (`self.Material`))
  (bind _returnvalue_2 (`KismetMaterialLibrary.CreateDynamicMaterialInstance` "/Game/HeeWon/MasterMaterial/MI_EdgeOutline_Test.MI_EdgeOutline_Test"))
  (set `self.Outliner` _returnvalue_2)
  (`SceneComponent.SetVisibility` (`self.Press F`) false false))

(event `self.ReceiveTick`
  (params (DeltaSeconds :type "Float (single-precision)"))
  (bind _material (`self.Material`))
  (`|ExecutionSequence`
    (:`then_0`
      ; 2페이즈되면 흐르는 그림
      (bind _asgsc (cast `/Game/HeeWon/BP/GSC` (`GameplayStatics.GetGameState`)))
      (if (`/Game/HeeWon/BP/GSC.state2?` _asgsc)
        (`/Engine/EditorBlueprintResources/StandardMacros.DoOnce` false
          (:`Completed`
            (`ActorComponent.K2_DestroyComponent` (`self.Box`))
            (bind (_direction _xspeed1 _yspeed1 _xspeed2 _yspeed2 _emissive _dissolve) (`Timeline|Move`)
              (:`Update`
                (`MaterialInstanceDynamic.SetScalarParameterValue` _material "XSpeed1" _xspeed1)
                (`MaterialInstanceDynamic.SetScalarParameterValue` _material "YSpeed1" _yspeed1)
                (`MaterialInstanceDynamic.SetScalarParameterValue` _material "XSpeed2" _xspeed2)
                (`MaterialInstanceDynamic.SetScalarParameterValue` _material "YSpeed2" _yspeed2)
                (`MaterialInstanceDynamic.SetScalarParameterValue` _material "Emissive" _emissive)
                (`MaterialInstanceDynamic.SetScalarParameterValue` _material "Dissolve" _dissolve)))))))
    (:`then_1`
      ; 위젯이 항상 나를 쳐다보게
      (`SceneComponent.K2_SetWorldRotation` (`self.Press F`) (`KismetMathLibrary.MakeRotator` 0.0 0.0 (+ (.yaw (`KismetMathLibrary.FindLookAtRotation` (`PlayerCameraManager.GetCameraLocation` (`GameplayStatics.GetPlayerCameraManager` 0)) (`self.K2_GetActorLocation`))) 180.0)) false false))
    (:`then_2`
      (bind _asgsc_2 (cast `/Game/HeeWon/BP/GSC` (`GameplayStatics.GetGameState`)))
      (if (`/Game/HeeWon/BP/GSC.state5?` _asgsc_2)
        (`/Engine/EditorBlueprintResources/StandardMacros.DoOnce` false
          (:`Completed`
            (`ActorComponent.SetActive` (`self.Niagara`) true false)
            (`ActorComponent.SetActive` (`self.Niagara1`) true false)
            (`SceneComponent.SetVisibility` (`self.PointLight`) true false)))))))

(event `/Game/HeeWon/BP/BPI_Interaction.Overlap`
  (bind _outliner (`self.Outliner`))
  (bind _weightedblendables_array (break `WeightedBlendables` (break `PostProcessSettings` (`PostProcessVolume.Settings` (`self.postprocess`)))))
  ; UI대화
  (`|ExecutionSequence`
    (:`then_0`
      (`SceneComponent.SetVisibility` (`self.Press F`) true false)
      (`PrimitiveComponent.SetRenderCustomDepth` (`self.Plane`) true))
    (:`then_1`
      (bind (_direction _intensity) (`Timeline|Timeline` :!label _label)
        (:`Update`
          (`MaterialInstanceDynamic.SetScalarParameterValue` _outliner "LineWidth" _intensity))))
    (:`then_2`
      (`KismetArrayLibrary.Array_Set` _weightedblendables_array 0 (make `WeightedBlendable` 1.0 _outliner)))))

(event `/Game/HeeWon/BP/BPI_Interaction.EndOverlap`
  ; UI대화
  (`WidgetLayoutLibrary.RemoveAllWidgets`)
  (`|ExecutionSequence`
    (:`then_0`
      (goto _label :!via `Stop`))
    (:`then_1`
      (`SceneComponent.SetVisibility` (`self.Press F`) false false)
      (`PrimitiveComponent.SetRenderCustomDepth` (`self.Plane`) false)
      ;; 엔드오버랩되면 UI꺼지게
      (set `self.ExistWBPTalk` false))))

(event `/Game/HeeWon/BP/BPI_Interaction.Fkey`
  ; UI인터렉션0번
  (if (`self.ExistWBPTalk`)
    (`Widget.RemoveFromParent` (stale _returnvalue))
    (set `self.ExistWBPTalk` false)
    (else
      (bind _returnvalue (`|CreateWidget` "/Game/HeeWon/Widget/WBP_Talk.WBP_Talk_C" null (`self.name`) (`self.talk`) null))
      (`UserWidget.AddToViewport` _returnvalue 0)
      (set `self.ExistWBPTalk` true))))

(fn `UserConstructionScript`)