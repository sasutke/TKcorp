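; Dialogue trigger actor that shows a WBP_Talk widget with its name, text and texture, freezing player movement on Overlap.
; Fkey closes the widget and restores walking, while EndOverlap clears all widgets and destroys the actor, making it one-shot.
; All three events switch on State: 1 always runs, while 2 to 4 require the matching State flag in the GSC game state.
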(event `/Game/HeeWon/BP/BPI_Interaction.Overlap`
  (bind _returnvalue (`GameplayStatics.GetGameState`))
  (switch `int` (`self.state`)
    (:`1`
      (bind _returnvalue_2 (`|CreateWidget` "/Game/HeeWon/Widget/WBP_Talk.WBP_Talk_C" null (`self.Name`) (`self.Full Text`) (`self.Texture`) :!label _label))
      (`UserWidget.AddToViewport` _returnvalue_2 0)
      (`CharacterMovementComponent.SetMovementMode` (`Character.CharacterMovement` (`GameplayStatics.GetPlayerCharacter` 0)) "MOVE_None" 0))
    (:`2`
      (bind _asgsc (cast `/Game/HeeWon/BP/GSC` _returnvalue))
      (if (`/Game/HeeWon/BP/GSC.state2?` _asgsc)
        (goto _label)))
    (:`3`
      (cast `/Game/HeeWon/BP/GSC` _returnvalue)
      (if (`/Game/HeeWon/BP/GSC.state3?` _asgsc)
        (goto _label)))
    (:`4`
      (bind _asgsc_2 (cast `/Game/HeeWon/BP/GSC` _returnvalue))
      (if (`/Game/HeeWon/BP/GSC.state4?` _asgsc_2)
        (goto _label)))))

(event `/Game/HeeWon/BP/BPI_Interaction.Fkey`
  (bind _returnvalue (`GameplayStatics.GetGameState`))
  (switch `int` (`self.state`)
    (:`1`
      (`Widget.RemoveFromParent` (stale `/Game/HeeWon/BP/BPI_Interaction.Overlap` _returnvalue_2) :!label _label_2)
      (`CharacterMovementComponent.SetMovementMode` (`Character.CharacterMovement` (`GameplayStatics.GetPlayerCharacter` 0)) "MOVE_Walking" 0))
    (:`2`
      (bind _asgsc (cast `/Game/HeeWon/BP/GSC` _returnvalue))
      (if (`/Game/HeeWon/BP/GSC.state2?` _asgsc)
        (goto _label_2)))
    (:`3`
      (cast `/Game/HeeWon/BP/GSC` _returnvalue)
      (if (`/Game/HeeWon/BP/GSC.state3?` _asgsc)
        (goto _label_2)))
    (:`4`
      (bind _asgsc_2 (cast `/Game/HeeWon/BP/GSC` _returnvalue))
      (if (`/Game/HeeWon/BP/GSC.state4?` _asgsc_2)
        (goto _label_2)))))

(event `/Game/HeeWon/BP/BPI_Interaction.EndOverlap`
  (bind _returnvalue (`GameplayStatics.GetGameState`))
  (switch `int` (`self.state`)
    (:`1`
      (`WidgetLayoutLibrary.RemoveAllWidgets`)
      (`self.K2_DestroyActor`))
    (:`2`
      (bind _asgsc (cast `/Game/HeeWon/BP/GSC` _returnvalue))
      (if (`/Game/HeeWon/BP/GSC.state2?` _asgsc)
        (`WidgetLayoutLibrary.RemoveAllWidgets`)
        (`self.K2_DestroyActor`)))
    (:`3`
      (cast `/Game/HeeWon/BP/GSC` _returnvalue)
      (if (`/Game/HeeWon/BP/GSC.state3?` _asgsc)
        (`WidgetLayoutLibrary.RemoveAllWidgets`)
        (`self.K2_DestroyActor`)))
    (:`4`
      (bind _asgsc_2 (cast `/Game/HeeWon/BP/GSC` _returnvalue))
      (if (`/Game/HeeWon/BP/GSC.state4?` _asgsc_2)
        (`WidgetLayoutLibrary.RemoveAllWidgets`)
        (`self.K2_DestroyActor`)))))

(fn `UserConstructionScript`
  (`parent.UserConstructionScript`))